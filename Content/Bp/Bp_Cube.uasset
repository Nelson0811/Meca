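; Interactable cube whose size changes with its height while the player is grabbing.
; Each tick during a grab, it compares its Z to the height saved at BeginPlay: above grows the mesh, otherwise it shrinks.
; The same step raises or lowers the player's physics-handle TargetDistance, with debug prints for each direction.
; The Interact interface event turns on physics simulation for the mesh.
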(event EventTick
  (params (DeltaSeconds :type Float%20%28single-precision%29))
  (bind _staticmesh (Variables|Default|GetStaticMesh))
  (bind _staticmesh_2 (Variables|Default|GetStaticMesh))
  (bind _distancemultiplayer (Variables|Default|GetDistanceMultiplayer))
  (bind _scalemultiplayer (Variables|Default|GetScaleMultiplayer))
  ;[1 1 1] EventTick
  ;;[1 0 0] savoir si le player prend l'objet
  (bind _asbp_third_person_character (Utilities|Casting|CastToBP_ThirdPersonCharacter (Game|GetPlayerCharacter 0)))
  (Variables|Default|SetPlayerRef _asbp_third_person_character)
  (if (Variables|/Game/ThirdPerson/Blueprints/BP_ThirdPersonCharacter.BP_ThirdPersonCharacter_C|GetIsGrab? _asbp_third_person_character)
    (if (> (.Z (Math|Vector|BreakVector (Transformation|GetActorLocation))) (Variables|Default|GetPreviousSize))
      ;;[0.002951 1 0] La hauteru est +
      (Development|PrintString "haut" true true "(R=0.000000,G=1.000000,B=0.311889,A=1.000000)")
      ;;;[1 0 0] je + le scale
      (Transformation|SetRelativeScale3D _staticmesh_2 (+ (Variables|/Script/Engine.SceneComponent|GetRelativeScale3D _staticmesh_2) (Math|Vector|MakeVector _scalemultiplayer _scalemultiplayer _scalemultiplayer)))
      ;;;[1 0 0] je + la distance di Ph du Player
      (Variables|/Game/ThirdPerson/Blueprints/BP_ThirdPersonCharacter.BP_ThirdPersonCharacter_C|SetTargetDistance (Variables|Default|GetPlayerRef) (+ (Variables|/Game/ThirdPerson/Blueprints/BP_ThirdPersonCharacter.BP_ThirdPersonCharacter_C|GetTargetDistance (Variables|Default|GetPlayerRef)) _distancemultiplayer))
      (else
        ;;[0.08516 1 0] La hauteur est -
        (Development|PrintString "bas" true true "(R=1.000000,G=0.396977,B=0.000000,A=1.000000)")
        ;;;[1 0 0] je - le scale
        (Transformation|SetRelativeScale3D _staticmesh (- (Variables|/Script/Engine.SceneComponent|GetRelativeScale3D _staticmesh) (Math|Vector|MakeVector _scalemultiplayer _scalemultiplayer _scalemultiplayer)))
        ;;;[1 0 0] je - la distance du physiqueHandle du player
        (Variables|/Game/ThirdPerson/Blueprints/BP_ThirdPersonCharacter.BP_ThirdPersonCharacter_C|SetTargetDistance (Variables|Default|GetPlayerRef) (- (Variables|/Game/ThirdPerson/Blueprints/BP_ThirdPersonCharacter.BP_ThirdPersonCharacter_C|GetTargetDistance (Variables|Default|GetPlayerRef)) _distancemultiplayer))))))

(event EventInteract
  ;[0.1704 1 0.2706] Interaction ( interface )
  (Development|PrintString "Hello")
  (Physics|SetSimulatePhysics (Variables|Default|GetStaticMesh) true))

(event EventBeginPlay
  ;[1 0.09687 0.09687] BeginPlay (Position original de l'acteur)
  (Variables|Default|SetPreviousSize (.Z (Math|Vector|BreakVector (Transformation|GetActorLocation)))))

(fn ConstructionScript)